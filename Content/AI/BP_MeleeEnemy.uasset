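; Melee axe-wielding enemy that chases ThirdPersonCharacter pawns spotted by PawnSensing and plays an attack montage on reaching them.
; AttackNotify plays a whoosh and damages characters overlapping DamageBox.
; ReceiveDamage lowers HP, reveals up to two blood components and calls Die, which plays scream and death montage, disables collision, heals the player and later destroys the actor.
; The construction script randomizes axe, hair, pants, shoes and body materials for visual variety.
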(event OnSeePawn(PawnSensing)
  (params (Pawn :type Pawn%20Object%20Reference))
  (if (Variables|Default|GetIsAlive?)
    (if (not (Variables|Default|GetIsAttacking?))
      (bind _asthird_person_character (Utilities|Casting|CastToThirdPersonCharacter Pawn))
      (AI|AIMoveTo self "0, 0, 0" _asthird_person_character 1e+02 false
        (:OnSuccess
          (if (not (Variables|Default|GetIsAttacking?))
            (Variables|Default|SetIsAttacking? true)
            (if (Variables|Default|GetIsAlive?)
              (bind _returnvalue (Animation|Montage|MontagePlay (Components|SkeletalMesh|GetAnimInstance (Variables|Character|GetMesh)) "/Game/Character/Animations/Attack/AM_Attack_01.AM_Attack_01" 1.1 "MontageLength" 0.0 true))
              (Utilities|FlowControl|Delay _returnvalue)
              (Variables|Default|SetIsAttacking? false))))))))

(event Custom|Die
  (bind _self self)
  (bind _mesh (Variables|Character|GetMesh))
  (Variables|Default|SetIsAlive? false)
  (Rendering|SetVisibility (Variables|Default|GetBlood01) false false)
  (Rendering|SetVisibility (Variables|Default|GetBlood02) false false)
  (Audio|PlaySoundatLocation "/Game/Sounds/OC_MaleScream.OC_MaleScream" (Transformation|GetWorldLocation (Variables|Character|GetMesh)) "0, 0, 0" (Math|Random|RandomFloatinRange 0.7 1.1) (Math|Random|RandomFloatinRange 0.8 1.3) 0.0 0 0 0)
  (bind _returnvalue (Animation|Montage|MontagePlay (Components|SkeletalMesh|GetAnimInstance (Variables|Character|GetMesh)) "/Game/AI/Melee/AM_Death_Brute_Right.AM_Death_Brute_Right" 1.0 "MontageLength" 0.0 true))
  (Utilities|FlowControl|Delay _returnvalue)
  (Class|SkeletalMeshComponent|SetEnableGravityonAllBodiesBelow _mesh false "None" true)
  (Physics|SetSimulatePhysics _mesh false)
  (Collision|SetCollisionEnabled (Variables|Collision|GetCapsuleComponent _self) "NoCollision")
  (Collision|SetCollisionEnabled (Variables|Character|GetMesh _self) "NoCollision")
  (bind _asthird_person_character (Utilities|Casting|CastToThirdPersonCharacter (Game|GetPlayerCharacter 0)))
  (Default|ReplenishHealth _asthird_person_character 15.0)
  (Utilities|FlowControl|Delay 3e+01)
  (Actor|DestroyActor))

(event Custom|AttackNotify
  (CallFunction|PlayWhooshSound)
  (for _array_element (Collision|GetOverlappingActors (Variables|Default|GetDamageBox) "/Game/ThirdPersonBP/Blueprints/ThirdPersonCharacter.ThirdPersonCharacter_C" :!class /Script/Engine.PrimitiveComponent)
    (bind _asthird_person_character (Utilities|Casting|CastToThirdPersonCharacter _array_element))
    (Default|ReceiveDamage _asthird_person_character (Variables|Default|GetDamage))))

(event Custom|PlayWhooshSound
  (Audio|PlaySoundatLocation "/Game/Sounds/Axe/Axtwoosh3.Axtwoosh3" (Transformation|GetWorldLocation (Variables|Character|GetMesh)) "0, 0, 0" 1.0 1.0 0.0 0 0 0))

(event EventBeginPlay)

(event EventTick
  (params (DeltaSeconds :type Float%20%28single-precision%29)))

(fn ConstructionScript
  (bind _mesh (Variables|Character|GetMesh))
  (bind _mesh_2 (Variables|Character|GetMesh))
  (bind _mesh_3 (Variables|Character|GetMesh))
  (bind _mesh_4 (Variables|Character|GetMesh))
  (bind _mesh_5 (Variables|Character|GetMesh))
  (Utilities|FlowControl|Sequence
    (:then_0
      ;[1 1 1] Axe
      (switch int (Math|Random|RandomIntegerinRange 0 5)
        (:0
          (Rendering|Material|SetMaterial _mesh_4 0 "/Game/AI/Melee/Mats/Axes/MI_Axe_Brown.MI_Axe_Brown"))
        (:1
          (Rendering|Material|SetMaterial _mesh_4 0 "/Game/AI/Melee/Mats/Axes/MI_Axe_DarkBlue.MI_Axe_DarkBlue"))
        (:2
          (Rendering|Material|SetMaterial _mesh_4 0 "/Game/AI/Melee/Mats/Axes/MI_Axe.MI_Axe"))
        (:3
          (Rendering|Material|SetMaterial _mesh_4 0 "/Game/AI/Melee/Mats/Axes/MI_Axe_LightBlue.MI_Axe_LightBlue"))
        (:4
          (Rendering|Material|SetMaterial _mesh_4 0 "/Game/AI/Melee/Mats/Axes/MI_Axe_LightGreen.MI_Axe_LightGreen"))
        (:5
          (Rendering|Material|SetMaterial _mesh_4 0 "/Game/AI/Melee/Mats/Axes/MI_Axe_LightPurple.MI_Axe_LightPurple"))))
    (:then_1
      ;[0.4533 1 0.3925] Hair
      (switch int (Math|Random|RandomIntegerinRange 0 6)
        (:0
          (Rendering|Material|SetMaterial _mesh_5 1 "/Game/AI/Melee/BaseMatInstances/M_Axe_BaseInst.M_Axe_BaseInst"))
        (:1
          (Rendering|Material|SetMaterial _mesh_5 1 "/Game/AI/Melee/Mats/Hair/MI_Hair_Black.MI_Hair_Black"))
        (:2
          (Rendering|Material|SetMaterial _mesh_5 1 "/Game/AI/Melee/Mats/Hair/MI_Hair_Blonde01.MI_Hair_Blonde01"))
        (:3
          (Rendering|Material|SetMaterial _mesh_5 1 "/Game/AI/Melee/Mats/Hair/MI_Hair_Blonde02.MI_Hair_Blonde02"))
        (:4
          (Rendering|Material|SetMaterial _mesh_5 1 "/Game/AI/Melee/Mats/Hair/MI_Hair_Red01.MI_Hair_Red01"))
        (:5
          (Rendering|Material|SetMaterial _mesh_5 1 "/Game/AI/Melee/Mats/Hair/MI_Hair_Red02.MI_Hair_Red02"))
        (:6
          (Rendering|Material|SetMaterial _mesh_5 1 "/Game/AI/Melee/BaseMatInstances/M_Hair_BaseInst.M_Hair_BaseInst"))))
    (:then_2
      ;[1 0.3925 0.4537] Pants
      (switch int (Math|Random|RandomIntegerinRange 0 6)
        (:0
          (Rendering|Material|SetMaterial _mesh_2 2 "/Game/AI/Melee/BaseMatInstances/M_Pants_BaseInst.M_Pants_BaseInst"))
        (:1
          (Rendering|Material|SetMaterial _mesh_2 2 "/Game/AI/Melee/Mats/Pants/MI_Brute_Bottom_Inst.MI_Brute_Bottom_Inst"))
        (:2
          (Rendering|Material|SetMaterial _mesh_2 2 "/Game/AI/Melee/Mats/Pants/MI_Pants_DarkBrown.MI_Pants_DarkBrown"))
        (:3
          (Rendering|Material|SetMaterial _mesh_2 2 "/Game/AI/Melee/Mats/Pants/MI_Pants_Red.MI_Pants_Red"))
        (:4
          (Rendering|Material|SetMaterial _mesh_2 2 "/Game/AI/Melee/Mats/Pants/MI_Pants_DarkRed.MI_Pants_DarkRed"))
        (:5
          (Rendering|Material|SetMaterial _mesh_2 2 "/Game/AI/Melee/Mats/Pants/MI_Pants_LightBrown.MI_Pants_LightBrown"))))
    (:then_3
      ;[1 0.7708 0.4098] Shoes
      (switch int (Math|Random|RandomIntegerinRange 1 5)
        (:0
          (Rendering|Material|SetMaterial _mesh_3 3 "/Game/AI/Melee/BaseMatInstances/M_Axe_BaseInst.M_Axe_BaseInst"))
        (:1
          (Rendering|Material|SetMaterial _mesh_3 3 "/Game/AI/Melee/BaseMatInstances/M_Shoes_BaseInst.M_Shoes_BaseInst"))
        (:2
          (Rendering|Material|SetMaterial _mesh_3 3 "/Game/AI/Melee/Mats/Shoes/MI_Shoes_Dark.MI_Shoes_Dark"))
        (:3
          (Rendering|Material|SetMaterial _mesh_3 3 "/Game/AI/Melee/Mats/Shoes/MI_Shoes_DarkBrown.MI_Shoes_DarkBrown"))
        (:4
          (Rendering|Material|SetMaterial _mesh_3 3 "/Game/AI/Melee/Mats/Shoes/MI_Shoes_Green.MI_Shoes_Green"))
        (:5
          (Rendering|Material|SetMaterial _mesh_3 3 "/Game/AI/Melee/Mats/Shoes/MI_Shoes_Red.MI_Shoes_Red"))))
    (:then_4
      ;[0.6452 0.6 1] Body
      (switch int (Math|Random|RandomIntegerinRange 0 6)
        (:0
          (Rendering|Material|SetMaterial _mesh 7 "/Game/AI/Melee/Mats/Body/MI_Body_DarkBrown.MI_Body_DarkBrown"))
        (:1
          (Rendering|Material|SetMaterial _mesh 7 "/Game/AI/Melee/Mats/Body/MI_Body_LightBrown.MI_Body_LightBrown"))
        (:2
          (Rendering|Material|SetMaterial _mesh 7 "/Game/AI/Melee/Mats/Body/MI_Body_LightGreen.MI_Body_LightGreen"))
        (:3
          (Rendering|Material|SetMaterial _mesh 7 "/Game/AI/Melee/Mats/Body/MI_Body_LightRed.MI_Body_LightRed"))
        (:4
          (Rendering|Material|SetMaterial _mesh 7 "/Game/AI/Melee/Mats/Body/MI_Body_LightYellow.MI_Body_LightYellow"))
        (:5
          (Rendering|Material|SetMaterial _mesh 7 "/Game/AI/Melee/Mats/Body/MI_Body_MediumRed.MI_Body_MediumRed"))))))

(fn ReceiveDamage
  (params (Damage :type Float%20%28single-precision%29))
  (bind _blood01 (Variables|Default|GetBlood01))
  (bind _blood02 (Variables|Default|GetBlood02))
  (if (Variables|Default|GetIsAlive?)
    (bind _output_get (Variables|Default|SetCurrentHP (- (Variables|Default|GetCurrentHP) Damage)))
    (if (<= _output_get 0.0)
      (CallFunction|Die)
      (elif (Variables|Default|GetAllowBlood?)
        (if (Rendering|IsVisible _blood01)
          (if (not (Rendering|IsVisible _blood02))
            (Rendering|SetVisibility _blood02 true false))
          (else
            (Rendering|SetVisibility _blood01 true false)))))))