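; Ranged enemy AI character that shoots arrows at the player character and can be damaged and killed.
; Pawn sensing turns it toward a seen ThirdPersonCharacter and plays the attack montage on a cooldown.
; A separate SpawnArrow event spawns Arrow_BP at the spawn point, then after a delay launches it along capsule forward with a velocity impulse.
; RecieveDmg reduces health and triggers Die, which plays a death montage, disables collision and later destroys the actor.
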(event OnSeePawn(PawnSensing)
  (params (Pawn :type Pawn%20Object%20Reference))
  (bind _asthird_person_character (Utilities|Casting|CastToThirdPersonCharacter Pawn))
  (if (Variables|Default|GetIsAlive?)
    (Utilities|FlowControl|Sequence
      (:then_0
        (Transformation|SetActorRotation (Math|Rotator|FindLookatRotation (Transformation|GetActorLocation) (Math|Vector|MakeVector (.X (Math|Vector|BreakVector (Transformation|GetActorLocation _asthird_person_character))) (.Y (Math|Vector|BreakVector (Transformation|GetActorLocation _asthird_person_character))) (.Z (Math|Vector|BreakVector (Transformation|GetActorLocation _asthird_person_character)))))))
      (:then_1
        (if (and (Variables|Default|GetIsAlive?) (Variables|Default|GetSpawnArrow?))
          (Animation|Montage|MontagePlay (Components|SkeletalMesh|GetAnimInstance (Variables|Character|GetMesh)) "/Game/AI/Archer/Animations/Attack/RangedAttack.RangedAttack" 1.0 "MontageLength" 0.0 true)
          (Variables|Default|SetSpawnArrow? false)
          (Utilities|FlowControl|Delay 2.5)
          (Variables|Default|SetSpawnArrow? true))))))

(event Custom|SpawnArrow
  (bind _capsulecomponent (Variables|Collision|GetCapsuleComponent))
  (bind _arrowspawnlocation (Variables|Default|GetArrowSpawnLocation))
  (Utilities|FlowControl|Delay 0.25)
  (Utilities|IsValid _arrowspawnlocation
    (:Is%20Valid
      (bind _returnvalue (Game|SpawnActorfromClass "/Game/AI/Arrow_BP.Arrow_BP_C" (Transformation|GetWorldTransform _arrowspawnlocation) "AlwaysSpawn" 0 0))
      (Utilities|FlowControl|Delay 0.55)
      (Utilities|IsValid (Variables|/Game/AI/Arrow_BP.Arrow_BP_C|GetStaticMesh _returnvalue)
        (:Is%20Valid
          (Utilities|IsValid _capsulecomponent
            (:Is%20Valid
              (Physics|AddImpulse (Variables|/Game/AI/Arrow_BP.Arrow_BP_C|GetStaticMesh _returnvalue) (* (Math|Vector|GetForwardVector _capsulecomponent) (Variables|Default|GetShotSpeed)) "None" true))))))))

(event Custom|Die
  (bind _self self)
  (bind _mesh (Variables|Character|GetMesh))
  (Variables|Default|SetIsAlive? false)
  (bind _returnvalue (Animation|Montage|MontagePlay (Components|SkeletalMesh|GetAnimInstance (Variables|Character|GetMesh)) "/Game/AI/Archer/Animations/Death/Death01.Death01" 1.0 "MontageLength" 0.0 true))
  (Utilities|FlowControl|Delay _returnvalue)
  (Class|SkeletalMeshComponent|SetEnableGravityonAllBodiesBelow _mesh false "None" true)
  (Physics|SetSimulatePhysics _mesh false)
  (Collision|SetCollisionEnabled (Variables|Collision|GetCapsuleComponent _self) "NoCollision")
  (Collision|SetCollisionEnabled (Variables|Character|GetMesh _self) "NoCollision")
  (Utilities|FlowControl|Delay 3e+01)
  (Actor|DestroyActor))

(fn ConstructionScript)

(fn RecieveDmg
  (params (damage :type Float%20%28single-precision%29))
  (bind _output_get (Variables|Default|SetCurrentHP (- (Variables|Default|GetCurrentHP) damage)))
  (if (<= _output_get 0.0)
    (CallFunction|Die)))