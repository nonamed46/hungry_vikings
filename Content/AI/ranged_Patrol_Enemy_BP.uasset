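; Ranged enemy Blueprint that turns to face a seen ThirdPersonCharacter and shoots arrows at it.
; Pawn sensing aims the actor above the player's origin, then spawns Arrow_BP and launches it by velocity-change impulse along the mesh's forward vector, throttled by a delayed flag.
; BeginPlay caches three patrol point locations and picks one randomly, but the timeline that would lerp between them is never triggered, so patrolling does not run.
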(event OnSeePawn(PawnSensing)
  (params (Pawn :type Pawn%20Object%20Reference))
  ;[0.4585 0.694 1] Facing Player and Shooting Behaviour
  (bind _asthird_person_character (Utilities|Casting|CastToThirdPersonCharacter Pawn))
  (Utilities|FlowControl|Sequence
    (:then_0
      (Transformation|SetActorRotation (Math|Rotator|FindLookatRotation (Transformation|GetActorLocation) (Math|Vector|MakeVector (.X (Math|Vector|BreakVector (Transformation|GetActorLocation _asthird_person_character))) (.Y (Math|Vector|BreakVector (Transformation|GetActorLocation _asthird_person_character))) (+ (.Z (Math|Vector|BreakVector (Transformation|GetActorLocation _asthird_person_character))) 1e+02)))))
    (:then_1
      (if (Variables|Default|GetSpawnArrow?)
        (bind _returnvalue (Game|SpawnActorfromClass "/Game/AI/Arrow_BP.Arrow_BP_C" (Transformation|GetWorldTransform (Variables|Default|GetArrowSpawnLocation)) "Undefined" 0 0))
        (Physics|AddImpulse (Variables|/Game/AI/Arrow_BP.Arrow_BP_C|GetStaticMesh _returnvalue) (* (Math|Vector|GetForwardVector (Variables|Character|GetMesh)) (Variables|Default|GetShotSpeed)) "None" true)
        (Variables|Default|SetSpawnArrow? false)
        (Utilities|FlowControl|Delay 2.0)
        (Variables|Default|SetSpawnArrow? true)))))

(event EventBeginPlay
  ;[1 0.7962 0.1085] Set PatrolPoints on BeginPlay
  (Variables|Default|SetPatrolPoints (Utilities|Array|MakeArray (Transformation|GetWorldLocation (Variables|Default|GetPatrolPoint0)) (Transformation|GetWorldLocation (Variables|Default|GetPatrolPoint1)) (Transformation|GetWorldLocation (Variables|Default|GetPatrolPoint2))))
  (CallFunction|GetRandomPatrolPoint))

(fn ConstructionScript)

(fn GetRandomPatrolPoint
  (Variables|Default|SetCurrentPatrolPoint (Math|Random|RandomInteger (Utilities|Array|Length (Variables|Default|GetPatrolPoints)))))