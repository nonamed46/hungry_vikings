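; Enemy archer AI that shoots physics arrows at the player, with randomized bow, outfit and body materials.
; Pawn sensing updates rotation and target distance through a helper, then plays the attack montage on a cooldown.
; SpawnArrow launches a BP_Arrow by forward impulse, adding distance-based lift for range.
; Damage reveals up to two blood effects; death plays sound and montage, disables collision, heals the player and expires the actor.
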(event OnSeePawn(PawnSensing)
  (params (Pawn :type Pawn%20Object%20Reference))
  (bind (_rotation _distance_metres_) (CallFunction|CalculateRoatationandDistancetoPlayer))
  (Utilities|Casting|CastToThirdPersonCharacter Pawn)
  (if (Variables|Default|GetbAlive)
    (Utilities|FlowControl|Sequence
      (:then_0
        (Transformation|SetActorRotation _rotation)
        (Variables|Default|SetTargetDistanceM _distance_metres_))
      (:then_1
        (if (and (Variables|Default|GetbAlive) (Variables|Default|GetbSpawnArrow))
          (Animation|Montage|PlayMontage (Variables|Character|GetMesh) "/Game/AI/Archer/Animations/Attack/AM_RangedAttack.AM_RangedAttack"
            (:then
              (Variables|Default|SetbSpawnArrow false)
              (Utilities|FlowControl|Delay 2.5)
              (Variables|Default|SetbSpawnArrow true))))))))

(event Custom|SpawnArrow
  (bind _capsulecomponent (Variables|Collision|GetCapsuleComponent))
  (bind _arrowspawnlocation (Variables|Default|GetArrowSpawnLocation))
  (bind _returnvalue (Math|Vector|GetForwardVector _capsulecomponent))
  (bind (_x _y _z) (Math|Vector|BreakVector _returnvalue))
  (Utilities|FlowControl|Delay 0.25)
  (Utilities|IsValid _arrowspawnlocation
    (:Is%20Valid
      (bind _returnvalue_2 (Game|SpawnActorfromClass "/Game/AI/BP_Arrow.BP_Arrow_C" (Transformation|GetWorldTransform _arrowspawnlocation) "AlwaysSpawn" 0 0))
      (Utilities|FlowControl|Delay 0.55)
      (Utilities|IsValid (Variables|/Game/AI/BP_Arrow.BP_Arrow_C|GetStaticMesh _returnvalue_2)
        (:Is%20Valid
          (Utilities|IsValid _capsulecomponent
            (:Is%20Valid
              (if (Physics|IsSimulatingPhysics (Variables|/Game/AI/BP_Arrow.BP_Arrow_C|GetStaticMesh _returnvalue_2) "None")
                (Physics|AddImpulse (Variables|/Game/AI/BP_Arrow.BP_Arrow_C|GetStaticMesh _returnvalue_2) (* (Math|Vector|MakeVector _x _y (+ _z (/ (* (Variables|Default|GetTargetDistanceM) 1.5e+02) (* (Variables|Default|GetShotSpeed) 1e+01)))) (Variables|Default|GetShotSpeed)) "None" true)
                (else
                  (Actor|DestroyActor _returnvalue_2))))))))))

(event Custom|Die
  (bind _self self)
  (bind _mesh (Variables|Character|GetMesh))
  (Variables|Default|SetbAlive false)
  (Rendering|SetVisibility (Variables|Default|GetBlood01) false false)
  (Rendering|SetVisibility (Variables|Default|GetBlood02) false false)
  (Audio|PlaySoundatLocation "/Game/Sounds/Yudena_argh.Yudena_argh" (Transformation|GetWorldLocation (Variables|Character|GetMesh)) "0, 0, 0" (Math|Random|RandomFloatinRange 0.7 1.1) (Math|Random|RandomFloatinRange 0.8 1.3) 0.0 0 0 0)
  (bind _returnvalue (Animation|Montage|MontagePlay (Components|SkeletalMesh|GetAnimInstance (Variables|Character|GetMesh)) "/Game/AI/Archer/Animations/Death/Death01.Death01" 1.0 "MontageLength" 0.0 true))
  (Utilities|FlowControl|Delay _returnvalue)
  (Class|SkeletalMeshComponent|SetEnableGravityonAllBodiesBelow _mesh false "None" true)
  (Physics|SetSimulatePhysics _mesh false)
  (Collision|SetCollisionEnabled (Variables|Collision|GetCapsuleComponent _self) "NoCollision")
  (Collision|SetCollisionEnabled (Variables|Character|GetMesh _self) "NoCollision")
  (bind _asthird_person_character (Utilities|Casting|CastToThirdPersonCharacter (Game|GetPlayerCharacter 0)))
  (Default|ReplenishHealth _asthird_person_character 1e+01)
  (Actor|SetLifeSpan 3e+01))

(fn ConstructionScript
  (Utilities|FlowControl|Sequence
    (:then_0
      ;[1 1 1] Bow
      (Rendering|Material|SetMaterial (Variables|Character|GetMesh) 0 (CallFunction|GetRandomBowColor)))
    (:then_1
      ;[1 1 1] Outfit
      (Rendering|Material|SetMaterial (Variables|Character|GetMesh) 1 (CallFunction|GetRandomClothingColor)))
    (:then_2
      ;[1 1 1] Body
      (Rendering|Material|SetMaterial (Variables|Character|GetMesh) 4 (CallFunction|GetRandomBodyColor)))))

(fn RecieveDmg
  (params (damage :type Float%20%28single-precision%29))
  (bind _blood01 (Variables|Default|GetBlood01))
  (bind _blood02 (Variables|Default|GetBlood02))
  (if (Variables|Default|GetbAlive)
    (bind _output_get (Variables|Default|SetCurrentHP (- (Variables|Default|GetCurrentHP) damage)))
    (if (<= _output_get 0.0)
      (CallFunction|Die)
      (elif (Variables|Default|GetbAllowBlood)
        (if (Rendering|IsVisible _blood01)
          (if (not (Rendering|IsVisible _blood02))
            (Rendering|SetVisibility _blood02 true false))
          (else
            (Rendering|SetVisibility _blood01 true false)))))))

(fn GetRandomBowColor
  (return (Utilities|Select :Index (Math|Random|RandomIntegerinRange 0 5) :Option%200 "/Game/AI/Archer/Materials/BaseMatInstances/MI_Akai_Bow_Base.MI_Akai_Bow_Base" :Option%201 "/Game/AI/Archer/Materials/MatInstances/MI_Akai_Bow_Dark.MI_Akai_Bow_Dark" :Option%202 "/Game/AI/Archer/Materials/MatInstances/MI_Akai_Bow_Green.MI_Akai_Bow_Green" :Option%203 "/Game/AI/Archer/Materials/MatInstances/MI_Akai_Bow_Red.MI_Akai_Bow_Red" :Option%204 "/Game/AI/Archer/Materials/MatInstances/MI_Akai_Bow_Red02.MI_Akai_Bow_Red02" :Option%205 "/Game/AI/Archer/Materials/MatInstances/MI_Akai_Bow_Yellow.MI_Akai_Bow_Yellow")))

(fn GetRandomClothingColor
  (return (Utilities|Select :Index (Math|Random|RandomIntegerinRange 0 6) :Option%200 "/Game/AI/Archer/Materials/BaseMatInstances/MI_Akai_Outfit_Base.MI_Akai_Outfit_Base" :Option%201 "/Game/AI/Archer/Materials/MatInstances/MI_Akai_Outfit_Blue.MI_Akai_Outfit_Blue" :Option%202 "/Game/AI/Archer/Materials/MatInstances/MI_Akai_Outfit_Brown.MI_Akai_Outfit_Brown" :Option%203 "/Game/AI/Archer/Materials/MatInstances/MI_Akai_Outfit_Dark.MI_Akai_Outfit_Dark" :Option%204 "/Game/AI/Archer/Materials/MatInstances/MI_Akai_Outfit_DarkGreen.MI_Akai_Outfit_DarkGreen" :Option%205 "/Game/AI/Archer/Materials/MatInstances/MI_Akai_Outfit_Red.MI_Akai_Outfit_Red")))

(fn GetRandomBodyColor
  (return (Utilities|Select :Index (Math|Random|RandomIntegerinRange 0 4) :Option%200 "/Game/AI/Archer/Materials/BaseMatInstances/MI_Akai_Body_Base.MI_Akai_Body_Base" :Option%201 "/Game/AI/Archer/Materials/MatInstances/MI_Akai_Body_Brown.MI_Akai_Body_Brown" :Option%202 "/Game/AI/Archer/Materials/MatInstances/MI_Akai_Body_DarkBrown.MI_Akai_Body_DarkBrown" :Option%203 "/Game/AI/Archer/Materials/MatInstances/MI_Akai_Body_Red.MI_Akai_Body_Red" :Option%204 "/Game/AI/Archer/Materials/MatInstances/MI_Akai_Body_Yellow.MI_Akai_Body_Yellow")))

(fn CalculateRoatationandDistancetoPlayer
  (bind _returnvalue (Transformation|GetActorLocation))
  (bind _returnvalue_2 (Transformation|GetActorLocation))
  (bind _returnvalue_3 (Math|Rotator|FindLookatRotation _returnvalue _returnvalue_2))
  (return (Math|Rotator|MakeRotator (Math|Float|Clamp(Float) (.roll _returnvalue_3) -2e+01 2e+01) (Math|Float|Clamp(Float) (.pitch _returnvalue_3) -2e+01 2e+01) (.yaw _returnvalue_3)) (/ (Math|Vector|Distance(Vector) _returnvalue _returnvalue_2) 1e+02)))