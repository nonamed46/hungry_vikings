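; Basic melee enemy AI character that chases and attacks the player on sight.
; Pawn sensing triggers an AI move to the player, then an attack montage whose AttackNotify damages players overlapping DamageBox.
; ReceiveDamage lowers HP and progressively shows two blood effects when allowed.
; Death hides blood, plays a montage, disables collision, heals the player and destroys the actor after a delay.
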(event OnSeePawn(PawnSensing)
  (params (Pawn :type Pawn%20Object%20Reference))
  (if (Variables|Default|GetIsAlive?)
    (if (not (Variables|Default|GetIsAttacking?))
      (bind _asthird_person_character (Utilities|Casting|CastToThirdPersonCharacter Pawn))
      (AI|AIMoveTo self "0, 0, 0" _asthird_person_character 1e+02 false
        (:OnSuccess
          (if (not (Variables|Default|GetIsAttacking?))
            (Variables|Default|SetIsAttacking? true)
            (if (Variables|Default|GetIsAlive?)
              (bind _returnvalue (Animation|Montage|MontagePlay (Components|SkeletalMesh|GetAnimInstance (Variables|Character|GetMesh)) "/Game/Character/Animations/Attack/Attack_01.Attack_01" 1.0 "MontageLength" 0.0 true))
              (Utilities|FlowControl|Delay _returnvalue)
              (Variables|Default|SetIsAttacking? false))))))))

(event Custom|Die
  (bind _self self)
  (bind _mesh (Variables|Character|GetMesh))
  (Variables|Default|SetIsAlive? false)
  (Rendering|SetVisibility (Variables|Default|GetBlood01) false false)
  (Rendering|SetVisibility (Variables|Default|GetBlood02) false false)
  (bind _returnvalue (Animation|Montage|MontagePlay (Components|SkeletalMesh|GetAnimInstance (Variables|Character|GetMesh)) "/Game/AI/Melee/Death_Brute_Right.Death_Brute_Right" 1.0 "MontageLength" 0.0 true))
  (Utilities|FlowControl|Delay _returnvalue)
  (Class|SkeletalMeshComponent|SetEnableGravityonAllBodiesBelow _mesh false "None" true)
  (Physics|SetSimulatePhysics _mesh false)
  (Collision|SetCollisionEnabled (Variables|Collision|GetCapsuleComponent _self) "NoCollision")
  (Collision|SetCollisionEnabled (Variables|Character|GetMesh _self) "NoCollision")
  (bind _asthird_person_character (Utilities|Casting|CastToThirdPersonCharacter (Game|GetPlayerCharacter 0)))
  (Default|ReplenishHealth _asthird_person_character 2e+01)
  (Utilities|FlowControl|Delay 3e+01)
  (Actor|DestroyActor))

(event Custom|AttackNotify
  (for _array_element (Collision|GetOverlappingActors (Variables|Default|GetDamageBox) "/Game/ThirdPersonBP/Blueprints/ThirdPersonCharacter.ThirdPersonCharacter_C" :!class /Script/Engine.PrimitiveComponent)
    (bind _asthird_person_character (Utilities|Casting|CastToThirdPersonCharacter _array_element))
    (Default|ReceiveDamage _asthird_person_character (Variables|Default|GetDamage))))

(event EventBeginPlay)

(event EventTick
  (params (DeltaSeconds :type Float%20%28single-precision%29)))

(fn ConstructionScript)

(fn ReceiveDamage
  (params (Damage :type Float%20%28single-precision%29))
  (bind _blood01 (Variables|Default|GetBlood01))
  (bind _blood02 (Variables|Default|GetBlood02))
  (if (Variables|Default|GetIsAlive?)
    (bind _output_get (Variables|Default|SetCurrentHP (- (Variables|Default|GetCurrentHP) Damage)))
    (if (<= _output_get 0.0)
      (CallFunction|Die)
      (elif (Variables|Default|GetAllowBlood?)
        (if (Rendering|IsVisible _blood01)
          (if (not (Rendering|IsVisible _blood02))
            (Rendering|SetVisibility _blood02 true false))
          (else
            (Rendering|SetVisibility _blood01 true false)))))))