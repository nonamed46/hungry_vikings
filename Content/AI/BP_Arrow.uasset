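; BP_Arrow is an enemy arrow projectile that damages the third-person player on hit.
; After a short delay on BeginPlay, it enables physics and gravity and arms itself.
; Mesh hits damage the player only while armed and the player is not attacking, and ignore archers and other arrows.
; Damaging the player or hitting anything else disarms it, disables physics and collision, then destroys it after a target-dependent delay.
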(event OnComponentHit(StaticMesh)
  (params (HitComponent :type Primitive%20Component%20Object%20Reference) (OtherActor :type Actor%20Object%20Reference) (OtherComp :type Primitive%20Component%20Object%20Reference) (NormalImpulse :type Vector :default "0, 0, 0") (Hit :type Hit%20Result%20Structure%20%28by%20ref%29))
  (bind _staticmesh (Variables|Default|GetStaticMesh))
  (bind _staticmesh_2 (Variables|Default|GetStaticMesh))
  (bind _staticmesh_3 (Variables|Default|GetStaticMesh))
  (bind _asthird_person_character (Utilities|Casting|CastToThirdPersonCharacter OtherActor)
    (:then
      (if (Variables|Default|GetArmed?)
        (if (not (Variables|/Game/ThirdPersonBP/Blueprints/ThirdPersonCharacter.ThirdPersonCharacter_C|GetIsAttacking? _asthird_person_character))
          (Default|ReceiveDamage _asthird_person_character 1e+01)
          (Variables|Default|SetArmed? false)
          (Physics|SetSimulatePhysics _staticmesh false)
          (Collision|SetCollisionEnabled _staticmesh "NoCollision")
          (Utilities|FlowControl|Delay 0.2)
          (Actor|DestroyActor))))
    (:CastFailed
      (Utilities|Casting|CastToBP_Archer OtherActor
        (:CastFailed
          (Utilities|Casting|CastToBP_MeleeEnemy OtherActor
            (:then
              (Variables|Default|SetArmed? false)
              (Physics|SetSimulatePhysics _staticmesh_2 false)
              (Collision|SetCollisionEnabled _staticmesh_2 "NoCollision")
              (Utilities|FlowControl|Delay 0.5)
              (Actor|DestroyActor))
            (:CastFailed
              (Utilities|Casting|CastToBP_Arrow OtherActor
                (:CastFailed
                  (Variables|Default|SetArmed? false)
                  (Physics|SetSimulatePhysics _staticmesh_3 false)
                  (Collision|SetCollisionEnabled _staticmesh_3 "NoCollision")
                  (Utilities|FlowControl|Delay 5.0)
                  (Actor|DestroyActor))))))))))

(event EventBeginPlay
  (bind _staticmesh (Variables|Default|GetStaticMesh))
  (Utilities|FlowControl|Delay 0.55)
  (Physics|SetSimulatePhysics _staticmesh true)
  (Physics|SetEnableGravity _staticmesh true)
  (Variables|Default|SetArmed? true))

(fn ConstructionScript)